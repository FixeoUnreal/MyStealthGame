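; BP_AIGuard is an AI guard with a random patrol routine and a widget showing its state.
; Patrol moves to a random PatrolPoints entry and repeats after a short delay on success, though nothing connected here starts it.
; OnGuardStateChanged sets the WBP_GuardState text to blank, "?" or "!" for Idle, Suspicious or Alerted.
; The hearing event is empty, and the StopMovement call is disconnected.
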(event OnHearNoise(PawnSensingComp)
  (params (Instigator :type Pawn%20Object%20Reference) (Location :type Vector%20%28by%20ref%29 :default "0, 0, 0") (Volume :type Float%20%28single-precision%29)))

(event Custom|Patrol
  (bind _patrolpoints (Variables|Default|GetPatrolPoints))
  (AI|AIMoveTo self "0, 0, 0" (Utilities|Array|Get(acopy) _patrolpoints (Math|Random|RandomInteger (Utilities|Array|Length _patrolpoints))) 5.0 false
    (:OnSuccess
      (Utilities|FlowControl|Delay 1.0)
      (CallFunction|Patrol))))

(event EventBeginPlay)

(event Collision|EventActorBeginOverlap
  (params (OtherActor :type Actor%20Object%20Reference)))

(event EventTick
  (params (DeltaSeconds :type Float%20%28single-precision%29)))

(event EventOnGuardStateChanged
  (params (NewState :type EAIState%20Enum :default "Idle"))
  (bind _aswbp_guard_state (Utilities|Casting|CastToWBP_GuardState (UserInterface|GetUserWidgetObject (Variables|Default|GetWidget_GuardState))))
  (Default|UpdateText _aswbp_guard_state (Utilities|Select :Index NewState :Idle "" :Suspicious "?" :Alerted "!")))

(fn ConstructionScript)